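; Actor component that adds timed wallrunning and wall jumping to its owning Character.
; TryWallrun line-traces right, then left, and on a hit derives the run direction from the wall normal and up vector.
; While running, Tick adds movement input and pins the starting height, without rechecking the wall.
; A timer or repeat TryWallrun call ends the run in Falling mode, the latter first launching the character.
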(event EventBeginPlay
  (bind _ascharacter (Utilities|Casting|CastToCharacter (Components|GetOwner)))
  (Variables|Default|Setowner _ascharacter))

(event EventTick
  (params (DeltaSeconds :type Float%20%28single-precision%29))
  (bind _owner (Variables|Default|Getowner))
  (bind _returnvalue (Transformation|GetActorLocation _owner))
  (if (Variables|Default|GetbIsWallrunning)
    (Pawn|Input|AddMovementInput _owner (* (Variables|Default|GetwallrunDirection) (Variables|Default|GetwallrunSpeed)) 1.0 false)
    (Transformation|SetActorLocation _owner (Math|Vector|MakeVector (.x _returnvalue) (.y _returnvalue) (Variables|Default|GetstartZ)) false false)))

(fn TryWallrun
  (if (Variables|Default|GetbIsWallrunning)
    (CallFunction|WallJump)
    (CallFunction|StopWallrun)
    (else
      (bind (_outhit _returnvalue) (CallFunction|CheckWall (Variables|Default|Getowner) false))
      (if _returnvalue
        (LocalVariables|SetL_HitResult _outhit)
        (Variables|Default|SetbIsLeft false)
        (Variables|Default|SetwallNormal (.Normal (Collision|BreakHitResult (LocalVariables|GetL_HitResult))) :!label _label)
        (Variables|Default|SetwallrunDirection (* (Math|Float|SelectFloat 1.0 -1.0 (Variables|Default|GetbIsLeft)) (Math|Vector|CrossProduct (.Normal (Collision|BreakHitResult (LocalVariables|GetL_HitResult))) (Transformation|GetActorUpVector (Variables|Default|Getowner)))))
        (CallFunction|StartWallrun)
        (else
          (bind (_outhit_2 _returnvalue_2) (CallFunction|CheckWall (Variables|Default|Getowner) true))
          (if _returnvalue_2
            (LocalVariables|SetL_HitResult _outhit_2)
            (Variables|Default|SetbIsLeft true)
            (goto _label)))))))

(fn CheckWall
  (params (Actor :type Character%20Object%20Reference) (bIsLeft :type Boolean))
  (bind _returnvalue (Transformation|GetActorLocation Actor))
  (bind (_outhit _returnvalue_2) (Collision|LineTraceByChannel _returnvalue (+ _returnvalue (* (Math|Float|SelectFloat -1.0 1.0 bIsLeft) (* (Transformation|GetActorRightVector Actor) (Variables|Default|GetwallCheckDistance)))) "TraceTypeQuery1" false 0 "None"))
  (return _outhit _returnvalue_2))

(fn StartWallrun
  (Variables|Default|SetstartZ (.z (Transformation|GetActorLocation (Variables|Default|Getowner))))
  (Utilities|Time|SetTimerbyFunctionName 0 "StopWallrun" (Variables|Default|GetmaxWallrunTime))
  (Variables|Default|SetbIsWallrunning true))

(fn StopWallrun
  (Pawn|Components|CharacterMovement|SetMovementMode (Variables|/Script/Engine.Character|GetCharacterMovement (Variables|Default|Getowner)) "MOVE_Falling" 0)
  (Variables|Default|SetbIsWallrunning false)
  (Utilities|Time|ClearTimerbyFunctionName 0 "StopWallrun"))

(fn WallJump
  (bind _wallnormal (Variables|Default|GetwallNormal))
  (bind _walljumpstrength (Variables|Default|GetwallJumpStrength))
  (bind _owner (Variables|Default|Getowner))
  (bind _returnvalue (Transformation|GetActorUpVector _owner))
  (Character|LaunchCharacter (Variables|Default|Getowner) (+ (+ (* (* _wallnormal -1.0) (.x _walljumpstrength)) (* (* (.y _walljumpstrength) (Math|Vector|CrossProduct _wallnormal _returnvalue)) (Math|Float|SelectFloat 1.0 -1.0 (Variables|Default|GetbIsLeft)))) (* (.z _walljumpstrength) _returnvalue)) true true))