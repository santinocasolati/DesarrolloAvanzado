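; Target lock component that finds an enemy in front of a supplied camera and tracks whether a lock is active.
; FindTarget sphere-traces along the camera's forward vector on the Visibility channel, accepting the hit actor only if it implements BPI_Enemy.
; TryLocking returns that actor when not already locked.
; StartLock and FinishLock only toggle the lock flag, without storing the target or moving the camera.
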(fn Setup
  (params (Camera :type Camera%20Component%20Object%20Reference))
  (Variables|Default|SetCamera Camera))

(fn TryLocking
  (if (not (Variables|Default|GetbIsLocking))
    (bind (_outhit _returnvalue) (CallFunction|FindTarget))
    (if _returnvalue
      (return (.HitActor (Collision|BreakHitResult _outhit))))))

(fn FindTarget
  (bind _camera (Variables|Default|GetCamera))
  (bind _returnvalue (Transformation|GetWorldLocation _camera))
  (bind _outhit (Collision|SphereTraceByChannel _returnvalue (+ _returnvalue (* (Math|Vector|GetForwardVector _camera) (Variables|Default|GetmaxDistance))) (Variables|Default|GetcheckRadius) "TraceTypeQuery1" false 0 "None"))
  (return _outhit (Utilities|DoesObjectImplementInterface (.HitActor (Collision|BreakHitResult _outhit)) "/Game/Blueprints/Enemies/BPI_Enemy.BPI_Enemy_C")))

(fn StartLock
  (Variables|Default|SetbIsLocking true))

(fn FinishLock
  (Variables|Default|SetbIsLocking false))