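; First-person player character Blueprint with movement, look, jump, wallrun and a target-lock dash.
; BPTargetLockComponent is set up with the camera and supplies the dash target, which a timeline lerps the character toward using swept location updates.
; Pressing jump while falling asks BPWallrunComponent to start a wallrun, which suppresses move input while active.
; A successful dash cancels any active wallrun and releases the lock when the timeline finishes.
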(event EventBeginPlay
  (Default|Setup (Variables|Default|GetBP_TargetLockComponent) (Variables|Default|GetFirstPersonCamera)))

(event Input|EnhancedActionEvents|EnhancedInputActionIA_Dash
  (params (ActionValue :type Boolean) (ElapsedSeconds :type Float%20%28double-precision%29) (TriggeredSeconds :type Float%20%28double-precision%29) (InputAction :type Input%20Action%20Object%20Reference :default "/Game/FirstPerson/Input/Actions/IA_Dash.IA_Dash"))
  (bind _bp_targetlockcomponent (Variables|Default|GetBP_TargetLockComponent))
  (bind _bp_wallruncomponent (Variables|Default|GetBP_WallrunComponent))
  (:Started
    (bind _hitactor (Default|TryLocking _bp_targetlockcomponent))
    (Utilities|IsValid _hitactor
      (:Is%20Valid
        (Default|StartLock _bp_targetlockcomponent)
        (if (Variables|/Game/Blueprints/WallRun/BP_WallrunComponent.BP_WallrunComponent_C|GetbIsWallrunning _bp_wallruncomponent)
          (Default|StopWallrun _bp_wallruncomponent))
        (Variables|Default|SetdashStartLocation (Transformation|GetActorLocation))
        (bind _alpha (Timeline|DashTimeline PlayFromStart)
          (:Update
            (Transformation|SetActorLocation (Math|Vector|Lerp(Vector) (Variables|Default|GetdashStartLocation) (Transformation|GetActorLocation _hitactor) _alpha) true false))
          (:Finished
            (Default|FinishLock (Variables|Default|GetBP_TargetLockComponent))))))))

(event Input|EnhancedActionEvents|EnhancedInputActionIA_Move
  (params (ActionValue :type Vector%202D%20Structure) (ElapsedSeconds :type Float%20%28double-precision%29) (TriggeredSeconds :type Float%20%28double-precision%29) (InputAction :type Input%20Action%20Object%20Reference :default "/Game/FirstPerson/Input/Actions/IA_Move.IA_Move"))
  (if (not (Variables|/Game/Blueprints/WallRun/BP_WallrunComponent.BP_WallrunComponent_C|GetbIsWallrunning (Variables|Default|GetBP_WallrunComponent)))
    (Pawn|Input|AddMovementInput (Transformation|GetActorRightVector) (.x ActionValue) false)
    (Pawn|Input|AddMovementInput (Transformation|GetActorForwardVector) (.y ActionValue) false)))

(event Input|EnhancedActionEvents|EnhancedInputActionIA_Look
  (params (ActionValue :type Vector%202D%20Structure) (ElapsedSeconds :type Float%20%28double-precision%29) (TriggeredSeconds :type Float%20%28double-precision%29) (InputAction :type Input%20Action%20Object%20Reference :default "/Game/FirstPerson/Input/Actions/IA_Look.IA_Look"))
  (Pawn|Input|AddControllerYawInput (.x ActionValue))
  (Pawn|Input|AddControllerPitchInput (.y ActionValue)))

(event Input|EnhancedActionEvents|EnhancedInputActionIA_Jump
  (params (ActionValue :type Boolean) (ElapsedSeconds :type Float%20%28double-precision%29) (TriggeredSeconds :type Float%20%28double-precision%29) (InputAction :type Input%20Action%20Object%20Reference :default "/Game/FirstPerson/Input/Actions/IA_Jump.IA_Jump"))
  (:Started
    (if (AI|Components|NavMovement|IsFalling (Variables|Character|GetCharacterMovement))
      (Default|TryWallrun (Variables|Default|GetBP_WallrunComponent))
      (else
        (Character|Jump))))
  (:Completed
    (Character|StopJumping)))

(fn ConstructionScript)